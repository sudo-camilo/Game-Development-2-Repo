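; Enemy actor that chases the player and damages them on touch.
; Tick offsets it toward the player pawn along a normalized X/Y direction scaled by Speed, without sweeping.
; Overlapping a myCharacter passes OnHitDamage to that character's ChangeHealth.
; Its own ChangeHealth clamps health, and at zero destroys the enemy, spawns a Coin in its place and plays a pitched-up collapse sound.
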(event `self.ReceiveActorBeginOverlap`
  (params (OtherActor :type "Actor Object Reference"))
  (bind _asmy_character (cast `/Game/Blueprints/myCharacter` OtherActor))
  (`/Game/Blueprints/myCharacter.ChangeHealth` _asmy_character (`self.onHitDamage`)))

(event `self.ReceiveHit`
  (params (MyComp :type "PrimitiveComponent Object Reference") (Other :type "Actor Object Reference") (OtherComp :type "PrimitiveComponent Object Reference") (bSelfMoved :type Boolean) (HitLocation :type "Vector Structure") (HitNormal :type "Vector Structure") (NormalImpulse :type "Vector Structure") (Hit :type "HitResult Structure (by ref)")))

(event `self.ReceiveTick`
  (params (DeltaSeconds :type "Float (single-precision)"))
  (bind (_returnvalue_x _returnvalue_y) (`KismetMathLibrary.BreakVector` (- (`self.K2_GetActorLocation` (`GameplayStatics.GetPlayerPawn` 0)) (`self.K2_GetActorLocation`))))
  (`self.K2_AddActorWorldOffset` (* (`KismetMathLibrary.Normal` (`KismetMathLibrary.MakeVector` _returnvalue_x _returnvalue_y)) (* DeltaSeconds (`self.speed`)))))

(fn `changeHealth`
  (params (changeInHealth :type Integer))
  (bind _output_get (set `self.health` (`KismetMathLibrary.Clamp` (+ (`self.health`) changeInHealth) 0 100)))
  (if (== _output_get 0)
    (`self.K2_DestroyActor`)
    (`|SpawnActorFromClass` "/Game/Blueprints/Coin.Coin_C" (`self.GetTransform`) "Undefined" "OverrideRootScale" null null)
    (`GameplayStatics.PlaySound2D` "/Game/StarterContent/Audio/Collapse02.Collapse02" 0.5 5.0 0.0 null null)))

(fn `UserConstructionScript`)