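; Projectile actor that damages and knocks back enemies it hits, and shrinks itself to a tenth scale on BeginPlay.
; On Hit, it passes its Damage value to an Enemy's ChangeHealth, then pushes that enemy's mesh along the inverted hit normal with a mass-independent force.
; A sequence also checks for Coin hits, but its final branch destroys the projectile on any hit.
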(event `self.ReceiveBeginPlay`
  (`self.SetActorScale3D` (0.1 0.1 0.1)))

(event `self.ReceiveHit`
  (params (MyComp :type "PrimitiveComponent Object Reference") (Other :type "Actor Object Reference") (OtherComp :type "PrimitiveComponent Object Reference") (bSelfMoved :type Boolean) (HitLocation :type "Vector Structure") (HitNormal :type "Vector Structure") (NormalImpulse :type "Vector Structure") (Hit :type "HitResult Structure (by ref)"))
  (`|ExecutionSequence`
    (:`then_0`
      (bind _asenemy (cast `/Game/Blueprints/Enemy` Other))
      (`/Game/Blueprints/Enemy.changeHealth` _asenemy (`self.damage`))
      (`/Engine/EditorBlueprintResources/StandardMacros.IsValid` _asenemy
        (:`Is Valid`
          (`PrimitiveComponent.AddForce` (`/Game/Blueprints/Enemy.StaticMesh` _asenemy) (* HitNormal -600000.0) "None" true)
          (`self.K2_DestroyActor`))))
    (:`then_1`
      (cast `/Game/Blueprints/Coin` Other)
      (`self.K2_DestroyActor`))
    (:`then_2`
      (`self.K2_DestroyActor`))))

(fn `UserConstructionScript`)